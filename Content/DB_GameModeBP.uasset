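; DB game mode Blueprint that assigns each player a team start and its team.
; The FindPlayerStart override gathers all DB_TeamStart actors and indexes them with an incrementing spawn counter, falling back to the first when that entry is invalid.
; It copies the chosen start's team onto the DB_PlayerController; the counter increments before lookup and is never reset here.
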(fn `FindPlayerStart`
  (params (Player :type "Controller Object Reference") (IncomingName :type String))
  (returns (ReturnValue :type "Actor Object Reference"))
  (locals (returnSpawn :type "DB_TeamStart Object Reference"))
  (bind _returnspawn (`local.returnSpawn`))
  (bind _spawnplayercount (`self.spawnPlayerCount`))
  (bind _outactors (`GameplayStatics.GetAllActorsOfClass` "/Script/DodgeBattle.DB_TeamStart"))
  (`/Engine/EditorBlueprintResources/StandardMacros.IncrementInt` _spawnplayercount
    (:`  `
      (bind _output (`|GetArrayItem` _outactors _spawnplayercount))
      (if (`KismetSystemLibrary.IsValid` _output)
        (set `local.returnSpawn` _output)
        (else
          (set `local.returnSpawn` (`|GetArrayItem` _outactors))))
      (bind _asdb_player_controller (cast `DB_PlayerController` Player)
        (:`then`
          (bind _returnvalue (`DB_TeamStart.GetTeam` _returnspawn))
          (`DB_PlayerController.SetTeam` _asdb_player_controller _returnvalue))
        (:`CastFailed`
          _))
      (return _returnspawn))))

(fn `UserConstructionScript`)